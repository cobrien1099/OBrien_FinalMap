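; SecretDoor_BP is a puzzle door that slides open when a first-person projectile strikes its symbol, revealing a lever according to its author comment.
; Hit or overlap on the symbol's collision box shares one projectile cast and name check, which plays a timeline.
; The timeline lerps the door's relative location from begin to end and shows the activated symbol light, hidden at BeginPlay.
; A character-triggered branch is left unconnected.
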(event OnComponentHit(BoxCollisionforSymbol)
  (params (HitComponent :type Primitive%20Component%20Object%20Reference) (OtherActor :type Actor%20Object%20Reference) (OtherComp :type Primitive%20Component%20Object%20Reference) (NormalImpulse :type Vector :default "0, 0, 0") (Hit :type Hit%20Result%20Structure%20%28by%20ref%29))
  ;[1 1 1] When the projectile hits the collisoin box, the door will slide open and reveal the lever
  (Utilities|Casting|CastToFirstPersonProjectile OtherActor)
  (if (Utilities|String|Contains (Utilities|GetDisplayName OtherActor) "projectile")
    (bind _door_open (Timeline|Secret%20Door%20Open Play)
      (:Update
        (Transformation|SetRelativeLocation (Variables|Default|GetSecret%20Door) (Math|Vector|Lerp(Vector) (Variables|Default|GetDoor%20Begin) (Variables|Default|GetDoor%20End) _door_open) false false)
        (Rendering|SetVisibility (Variables|Default|GetSymbol%20Light%20Activated) true false)))))

(event OnComponentBeginOverlap(BoxCollisionforSymbol)
  (params (OverlappedComponent :type Primitive%20Component%20Object%20Reference) (OtherActor :type Actor%20Object%20Reference) (OtherComp :type Primitive%20Component%20Object%20Reference) (OtherBodyIndex :type Integer) (bFromSweep :type Boolean) (SweepResult :type Hit%20Result%20Structure%20%28by%20ref%29))
  ;[1 1 1] When the projectile hits the collisoin box, the door will slide open and reveal the lever
  (Utilities|Casting|CastToFirstPersonProjectile (stale OnComponentHit(BoxCollisionforSymbol) OtherActor))
  (if (Utilities|String|Contains (Utilities|GetDisplayName (stale OnComponentHit(BoxCollisionforSymbol) OtherActor)) "projectile")
    (bind _door_open (Timeline|Secret%20Door%20Open Play)
      (:Update
        (Transformation|SetRelativeLocation (Variables|Default|GetSecret%20Door) (Math|Vector|Lerp(Vector) (Variables|Default|GetDoor%20Begin) (Variables|Default|GetDoor%20End) _door_open) false false)
        (Rendering|SetVisibility (Variables|Default|GetSymbol%20Light%20Activated) true false)))))

(event EventBeginPlay
  ;[1 1 1] Light Disappears At Start
  (Rendering|SetVisibility (Variables|Default|GetSymbol%20Light%20Activated) false false))

(event Collision|EventActorBeginOverlap
  (params (OtherActor :type Actor%20Object%20Reference)))

(event EventTick
  (params (DeltaSeconds :type Float%20%28single-precision%29)))

(fn ConstructionScript)