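; Text_BP is a proximity text prompt in a door puzzle project that appears while the player stands inside its trigger box.
; Begin and end overlap events on BoxCollision compare the overlapping actor with PlayerReference, then toggle WidgetText visibility and the CanInteract flag.
; The graph neither assigns PlayerReference nor reads CanInteract.
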(event OnComponentBeginOverlap(BoxCollision)
  (params (OverlappedComponent :type Primitive%20Component%20Object%20Reference) (OtherActor :type Actor%20Object%20Reference) (OtherComp :type Primitive%20Component%20Object%20Reference) (OtherBodyIndex :type Integer) (bFromSweep :type Boolean) (SweepResult :type Hit%20Result%20Structure%20%28by%20ref%29))
  ;[1 1 1] Blueprint Interacts with Player (Text Visible)
  (if (== OtherActor (Variables|Default|GetPlayer%20Reference))
    (Variables|Default|SetCan%20Interact true)
    (Rendering|SetVisibility (Variables|Default|GetWidget%20Text) true false)))

(event OnComponentEndOverlap(BoxCollision)
  (params (OverlappedComponent :type Primitive%20Component%20Object%20Reference) (OtherActor :type Actor%20Object%20Reference) (OtherComp :type Primitive%20Component%20Object%20Reference) (OtherBodyIndex :type Integer))
  ;[1 1 1] Blueprint Stops Interacting With Player (Invisible)
  (if (== (Variables|Default|GetPlayer%20Reference) OtherActor)
    (Variables|Default|SetCan%20Interact false)
    (Rendering|SetVisibility (Variables|Default|GetWidget%20Text) false false)))

(fn ConstructionScript)